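; Player character for a 2D side-scroller, handling movement, jumping, damage and talking to the guide NPC.
; Enhanced Input drives X-axis movement gated by CanMove and jumps that swap flipbooks on press and release; sprite-flip logic is present but unconnected.
; BeginPlay adds the mapping context and base UI.
; Interact shows the guide's dialogue widget if its PlayerInRange is set, otherwise removes it; damage subtracts from HP.
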(event Custom|SetUI_NPCGuide
  (bind _returnvalue (UserInterface|CreateWidget "/Game/1144c006_W03/NPC_Guide/Widget/UI_ForNPCGuide.UI_ForNPCGuide_C"))
  (Widget|SetVisibility (Variables|/Game/1144c006_W03/NPC_Guide/Widget/UI_ForNPCGuide.UI_ForNPCGuide_C|GetTxt_NPC_Talk _returnvalue) "Visible")
  (UserInterface|Viewport|AddtoViewport _returnvalue 0))

(event Custom|SET%20UI%20NPCGuide%20Remove
  (Widget|RemovefromParent (stale Custom|SetUI_NPCGuide _returnvalue)))

(event Custom|Set%20UI%20Base
  (bind _returnvalue (UserInterface|CreateWidget "/Game/1144c006_W03/BP_NPC_LookAround/UI_Base.UI_Base_C"))
  (UserInterface|Viewport|AddtoViewport _returnvalue 0))

(event Input|EnhancedActionEvents|EnhancedInputActionIA_Move01
  (params (ActionValue :type Vector%202D%20Structure) (ElapsedSeconds :type Float%20%28double-precision%29) (TriggeredSeconds :type Float%20%28double-precision%29) (InputAction :type Input%20Action%20Object%20Reference :default "/Game/1144c006_W03/Input/IA_Move01.IA_Move01"))
  (bind _x (Math|Vector2D|BreakVector2D ActionValue))
  (if (Variables|Default|GetCanMove)
    (if (> _x 0.0)
      (Variables|Default|SetIsFacingRight true)
      (else
        (Variables|Default|SetIsFacingRight false)))
    (Pawn|Input|AddMovementInput "1.000000,0.000000,0.000000" _x false)
    (else
      (Development|PrintString "Move Locked"))))

(event Input|EnhancedActionEvents|EnhancedInputActionIA_Jump01
  (params (ActionValue :type Boolean) (ElapsedSeconds :type Float%20%28double-precision%29) (TriggeredSeconds :type Float%20%28double-precision%29) (InputAction :type Input%20Action%20Object%20Reference :default "/Game/1144c006_W03/Input/IA_Jump01.IA_Jump01"))
  (:Started
    (Character|Jump)
    (Sprite|SetFlipbook (Variables|Default|GetPaperFlipbook) "/Game/U06/Flipbook/FB_Girl_Jump.FB_Girl_Jump"))
  (:Completed
    (Character|StopJumping)
    (Sprite|SetFlipbook (Variables|Default|GetPaperFlipbook) "/Game/U06/Flipbook/FB_Girl_Idle.FB_Girl_Idle")))

(event Input|EnhancedActionEvents|EnhancedInputActionIA_Interact
  (params (ActionValue :type Boolean) (ElapsedSeconds :type Float%20%28double-precision%29) (TriggeredSeconds :type Float%20%28double-precision%29) (InputAction :type Input%20Action%20Object%20Reference :default "/Game/1144c006_W03/Input/IA_Interact.IA_Interact"))
  (:Started
    (bind _returnvalue (Actor|GetActorOfClass "/Game/1144c006_W03/NPC_Guide/BP_NPC_Guide.BP_NPC_Guide_C"))
    (bind _asbp_npc_guide (Utilities|Casting|CastToBP_NPC_Guide _returnvalue))
    (if (Variables|/Game/1144c006_W03/NPC_Guide/BP_NPC_Guide.BP_NPC_Guide_C|GetPlayerInRange _asbp_npc_guide)
      (CallFunction|SetUINPCGuide)
      (else
        (Development|PrintString "NoNPC")
        (CallFunction|SETUINPCGuideRemove)))))

(event EventBeginPlay
  (Input|AddMappingContext (PlayerController|LocalPlayerSubsystems|GetEnhancedInputLocalPlayerSubsystem (Game|GetPlayerController 0)) "/Game/1144c006_W03/Input/IMC_Player.IMC_Player" 0 "(bIgnoreAllPressedKeysUntilRelease=True,bForceImmediately=False,bNotifyUserSettings=False)")
  (CallFunction|SetUIBase))

(event Collision|EventActorBeginOverlap
  (params (OtherActor :type Actor%20Object%20Reference)))

(event EventTick
  (params (DeltaSeconds :type Float%20%28single-precision%29)))

(event Game|Damage|EventAnyDamage
  (params (Damage :type Float%20%28single-precision%29) (DamageType :type Damage%20Type%20Object%20Reference) (InstigatedBy :type Controller%20Object%20Reference) (DamageCauser :type Actor%20Object%20Reference))
  (Variables|Default|SetHP (- (Variables|Default|GetHP) Damage)))

(fn ConstructionScript)